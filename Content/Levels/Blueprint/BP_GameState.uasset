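; BP_GameState is a game state Blueprint that tracks the scores of a red and a blue team.
; SetRedScore and SetBlueScore each add one point to their team's score and print the new total.
; BeginPlay creates a random stream from an initial seed, though nothing in these graphs draws from it.
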(event `self.ReceiveBeginPlay`
  (set `self.Stream` (`KismetMathLibrary.MakeRandomStream` (`self.Initial Seed`))))

(event `SetRedScore`
  ;[1 1 1] Score Red
  (bind _output_get (set `self.RedScore` (+ (`self.RedScore`) 1)))
  (`KismetSystemLibrary.PrintString` (`KismetStringLibrary.Conv_IntToString` _output_get)))

(event `SetBlueScore`
  ;[1 1 1] Score Blue
  (bind _output_get (set `self.BlueScore` (+ (`self.BlueScore`) 1)))
  (`KismetSystemLibrary.PrintString` (`KismetStringLibrary.Conv_IntToString` _output_get)))

(fn `UserConstructionScript`)