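; BP_Goal is a team goal actor that awards a point to the opposing team when the ball enters it.
; On BeginPlay it finds BP_Ball in the level and tints its three cube meshes red or blue from the Team enum.
; Box overlaps are handled only with authority: the ball entering updates the other side's score on BP_GameState, then calls MoveActor on the ball to reset it.
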(event `self.ReceiveBeginPlay`
  ;[1 1 1] Calls soft ref/ sets Goal colour based on Team Enum
  (bind _returnvalue (`GameplayStatics.GetActorOfClass` "/Game/Levels/Blueprint/BP_Ball.BP_Ball_C"))
  (set `self.Ball` _returnvalue)
  (switch `/Game/Levels/Blueprint/E_Teams` (`self.Team`)
    (:`NewEnumerator0`
      (`MeshComponent.SetVectorParameterValueOnMaterials` (`self.Cube`) "Colour" (1.0 0.0 0.0))
      (`MeshComponent.SetVectorParameterValueOnMaterials` (`self.Cube1`) "Colour" (1.0 0.0 0.0))
      (`MeshComponent.SetVectorParameterValueOnMaterials` (`self.Cube2`) "Colour" (1.0 0.0 0.0)))
    (:`NewEnumerator1`
      (`MeshComponent.SetVectorParameterValueOnMaterials` (`self.Cube`) "Colour" (0.0 0.0 1.0))
      (`MeshComponent.SetVectorParameterValueOnMaterials` (`self.Cube1`) "Colour" (0.0 0.0 1.0))
      (`MeshComponent.SetVectorParameterValueOnMaterials` (`self.Cube2`) "Colour" (0.0 0.0 1.0)))))

(event `self.Box.OnComponentBeginOverlap`
  (params (OverlappedComponent :type "PrimitiveComponent Object Reference") (OtherActor :type "Actor Object Reference") (OtherComp :type "PrimitiveComponent Object Reference") (OtherBodyIndex :type Integer) (bFromSweep :type Boolean) (SweepResult :type "HitResult Structure (by ref)"))
  (bind _ball (`self.Ball`))
  ;[1 1 1] Checks ball in goal and sets score to game state
  (`/Engine/EditorBlueprintResources/ActorMacros.Switch Has Authority`
    (:`Authority`
      (if (== OtherActor (`self.Ball`))
        (bind _asbp_game_state (cast `/Game/Levels/Blueprint/BP_GameState` (`GameplayStatics.GetGameState`)))
        ;[1 1 1] Scores point to correct side and resets ball position
        (switch `/Game/Levels/Blueprint/E_Teams` (`self.Team`)
          (:`NewEnumerator0`
            (`/Game/Levels/Blueprint/BP_GameState.SetBlueScore` _asbp_game_state)
            (`/Game/Levels/Blueprint/BP_Ball.MoveActor` _ball))
          (:`NewEnumerator1`
            (`/Game/Levels/Blueprint/BP_GameState.SetRedScore` _asbp_game_state)
            (`/Game/Levels/Blueprint/BP_Ball.MoveActor` _ball)))))))

(fn `UserConstructionScript`)