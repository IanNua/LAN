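; BP_Ball is a networked physics ball actor that can be reset to a fixed world position.
; MoveActor runs its reset only on the authority: it enables Sphere replication, turns physics off, teleports the sphere, then re-enables simulation.
; BeginPlay's authority check leads nowhere.
; CheckLocation ignores its parameter and forces a net update on player character 0.
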(event `MoveActor`
  (bind _sphere (`self.Sphere`))
  (`/Engine/EditorBlueprintResources/ActorMacros.Switch Has Authority`
    (:`Authority`
      ;[1 1 1] Resets position in ball, don't add delay...
      (`ActorComponent.SetIsReplicated` (`self.Sphere`) true)
      (`PrimitiveComponent.SetSimulatePhysics` _sphere false)
      (`SceneComponent.K2_SetWorldLocation` _sphere (0.0 -390.0 0.0) false true)
      (`PrimitiveComponent.SetSimulatePhysics` _sphere true))))

(event `self.ReceiveBeginPlay`
  ;[1 1 1] Sets Authority?
  (`/Engine/EditorBlueprintResources/ActorMacros.Switch Has Authority`))

(fn `CheckLocation`
  (params (NewParam :type "Vector Structure"))
  (`self.ForceNetUpdate` (`GameplayStatics.GetPlayerCharacter` 0)))

(fn `UserConstructionScript`)