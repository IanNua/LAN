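; Cluedo level pickup actor that holds a random object type and gives it to whoever touches it.
; On BeginPlay the authority picks one of three enum values, with the third twice as likely, and shows its name on a TextRender.
; Box overlap passes the value to the overlapping actor through UpdatePlayerObjMessage, then destroys the pickup, without an authority check.
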(event `self.ReceiveBeginPlay`
  (bind _textrender (`self.TextRender`))
  (`/Engine/EditorBlueprintResources/ActorMacros.Switch Has Authority`
    (:`Authority`
      (switch `int` (`KismetMathLibrary.RandomIntegerInRange` 0 3)
        (:`0`
          (bind _output_get (set `self.Objects` "NewEnumerator0"))
          (`TextRenderComponent.K2_SetText` _textrender (`KismetTextLibrary.Conv_StringToText` (`|GetEnumeratorNameAsString` _output_get))))
        (:`1`
          (bind _output_get_2 (set `self.Objects` "NewEnumerator1"))
          (`TextRenderComponent.K2_SetText` _textrender (`KismetTextLibrary.Conv_StringToText` (`|GetEnumeratorNameAsString` _output_get_2))))
        (:`2`
          (bind _output_get_3 (set `self.Objects` "NewEnumerator2"))
          (`TextRenderComponent.K2_SetText` _textrender (`KismetTextLibrary.Conv_StringToText` (`|GetEnumeratorNameAsString` _output_get_3))))
        (:`3`
          (bind _output_get_4 (set `self.Objects` "NewEnumerator2"))
          (`TextRenderComponent.K2_SetText` _textrender (`KismetTextLibrary.Conv_StringToText` (`|GetEnumeratorNameAsString` _output_get_4))))))))

(event `self.Box.OnComponentBeginOverlap`
  (params (OverlappedComponent :type "PrimitiveComponent Object Reference") (OtherActor :type "Actor Object Reference") (OtherComp :type "PrimitiveComponent Object Reference") (OtherBodyIndex :type Integer) (bFromSweep :type Boolean) (SweepResult :type "HitResult Structure (by ref)"))
  (message `/Game/Levels/Blueprint/Cluedo/BPI_UpdatePlayer.UpdatePlayerObj` OtherActor (`self.Objects`))
  (`self.K2_DestroyActor`))

(fn `UserConstructionScript`)